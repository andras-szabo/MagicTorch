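; Magic torch actor that snaps to the player's gun muzzle and toggles a light cone on input by lerping its FOV open or closed.
; FOV and length drive a scene capture, a box collision volume and, with the actor's transform, a Material Parameter Collection describing the cone to shaders.
; While lit, components entering the box switch collision channel, reverting on exit.
; Tick also draws a rotating debug-line cone.
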(event `self.ReceiveBeginPlay`
  ;[1 1 1] Setup on BeginPlay
  (set `self.MaxFOV` (`self.FOV`))
  (set `self.CurrentEndFOV` 0.0)
  (set `self.FOV` 0.0)
  (`self.ApplyTorchParameters`)
  (`self.GetGunSocket`))

(event `InputAction|Torch`
  (params (Key :type "Key Structure"))
  ;[1 1 1] Toggle torch based on input
  (:`Pressed`
    (`self.Toggle` (<= (`self.CurrentEndFOV`) 0.0))))

(event `self.CollisionVolume.OnComponentBeginOverlap`
  (params (OverlappedComponent :type "PrimitiveComponent Object Reference") (OtherActor :type "Actor Object Reference") (OtherComp :type "PrimitiveComponent Object Reference") (OtherBodyIndex :type Integer) (bFromSweep :type Boolean) (SweepResult :type "HitResult Structure (by ref)"))
  ;[1 1 1] Handle collisions
  (if (> (`self.FOV`) 0.0)
    (`PrimitiveComponent.SetCollisionObjectType` OtherComp "ECC_GameTraceChannel2")))

(event `self.ReceiveTick`
  (params (DeltaSeconds :type "Float (single-precision)"))
  (bind _conerolloffset (`self.ConeRollOffset`))
  ;[1 1 1] Update on Tick
  (if (!= (`self.CurrentEndFOV`) (`self.FOV`))
    (bind _output_get (set `self.ElapsedWhileChangingFOV` (+ (`self.ElapsedWhileChangingFOV`) DeltaSeconds)))
    (`self.AdjustFOV` (`KismetMathLibrary.Lerp` (`self.CurrentStartFOV`) (`self.CurrentEndFOV`) (`KismetMathLibrary.FClamp` (/ _output_get (`self.ToggleDuration`)))))
    (`self.ApplyTorchTransform`)
    (else
      (`self.ApplyTorchTransform`)))
  (if (> (`self.FOV`) 0.0)
    (`self.DebugDrawTorch` _conerolloffset)
    (set `self.ConeRollOffset` (mod (+ _conerolloffset 1) 360))))

(event `self.CollisionVolume.OnComponentEndOverlap`
  (params (OverlappedComponent :type "PrimitiveComponent Object Reference") (OtherActor :type "Actor Object Reference") (OtherComp :type "PrimitiveComponent Object Reference") (OtherBodyIndex :type Integer))
  ;[1 1 1] Handle collisions
  (`PrimitiveComponent.SetCollisionObjectType` OtherComp "ECC_GameTraceChannel1"))

(fn `AdjustFOV`
  (params (NewFOV :type "Float (double-precision)"))
  (set `self.FOV` NewFOV)
  (`self.ApplyTorchParameters`))

(fn `ApplyTorchParameters`
  (bind _collisionvolume (`self.CollisionVolume`))
  (bind _fov (`self.FOV`))
  (bind _length (`self.Length`))
  (bind _scenecapture (`self.SceneCapture`))
  (bind _returnvalue (/ (`self.Length`) 2.0))
  (bind _returnvalue_2 (/ _fov 2.0))
  (bind _returnvalue_3 (`KismetMathLibrary.DegTan` _returnvalue_2))
  (bind _returnvalue_4 (* _returnvalue_3 (/ (`self.Length`) 2.0)))
  (set `SceneCaptureComponent2D.FOVAngle` _fov _scenecapture)
  (set `SceneCaptureComponent.MaxViewDistanceOverride` _length _scenecapture)
  (`KismetMaterialLibrary.SetScalarParameterValue` "/Game/MagicTorch/Materials/TorchParameters.TorchParameters" "coneLength" _length)
  (`KismetMaterialLibrary.SetScalarParameterValue` "/Game/MagicTorch/Materials/TorchParameters.TorchParameters" "coneEdgeLength" (/ _length (`KismetMathLibrary.DegCos` _returnvalue_2)))
  (`KismetMaterialLibrary.SetScalarParameterValue` "/Game/MagicTorch/Materials/TorchParameters.TorchParameters" "zoom" (/ 1.0 _returnvalue_3))
  (`BoxComponent.SetBoxExtent` _collisionvolume (`KismetMathLibrary.MakeVector` _returnvalue _returnvalue_4 _returnvalue_4) true)
  (`SceneComponent.K2_SetWorldLocation` _collisionvolume (+ (* (`self.GetActorForwardVector`) _returnvalue) (`self.K2_GetActorLocation`)) false true))

(fn `ApplyTorchTransform`
  (bind _rotation (.rotation (`self.GetTransform`)))
  (`KismetMaterialLibrary.SetVectorParameterValue` "/Game/MagicTorch/Materials/TorchParameters.TorchParameters" "coneOriginWS" (`KismetMathLibrary.Conv_VectorToLinearColor` (.location (`self.GetTransform`))))
  (`KismetMaterialLibrary.SetVectorParameterValue` "/Game/MagicTorch/Materials/TorchParameters.TorchParameters" "coneForwardWS" (`KismetMathLibrary.Conv_VectorToLinearColor` (`KismetMathLibrary.GetForwardVector` _rotation)))
  (`KismetMaterialLibrary.SetVectorParameterValue` "/Game/MagicTorch/Materials/TorchParameters.TorchParameters" "coneRightWS" (`KismetMathLibrary.Conv_VectorToLinearColor` (`KismetMathLibrary.GetRightVector` _rotation)))
  (`KismetMaterialLibrary.SetVectorParameterValue` "/Game/MagicTorch/Materials/TorchParameters.TorchParameters" "coneUpWS" (`KismetMathLibrary.Conv_VectorToLinearColor` (`KismetMathLibrary.GetUpVector` _rotation))))

(fn `DebugDrawTorch`
  (params (RotationOffset :type Integer))
  (locals (TorchUp :type "Vector Structure") (TorchRight :type "Vector Structure") (StartPosition :type "Vector Structure") (ConeBaseCentre :type "Vector Structure") (BaseWidth :type "Float (double-precision)"))
  (bind _location (.location (`self.GetTransform`)))
  (bind _rotation (.rotation (`self.GetTransform`)))
  (set `local.BaseWidth` (* (`self.Length`) (`KismetMathLibrary.DegTan` (/ (`self.FOV`) 2.0))))
  (set `local.StartPosition` _location)
  (set `local.TorchUp` (* (`KismetMathLibrary.GetUpVector` _rotation) (`local.BaseWidth`)))
  (set `local.TorchRight` (* (`KismetMathLibrary.GetRightVector` _rotation) (`local.BaseWidth`)))
  (set `local.ConeBaseCentre` (+ _location (* (`KismetMathLibrary.GetForwardVector` _rotation) (`self.Length`))))
  (for _index (range 4)
    (for _index_2 (range 1 4)
      (bind _returnvalue (+ (+ (* (`KismetMathLibrary.Conv_IntToDouble` _index_2) (/ 90.0 3.0)) (* _index 90.0)) (`KismetMathLibrary.Conv_IntToDouble` RotationOffset)))
      (`KismetSystemLibrary.DrawDebugLine` (`local.StartPosition`) (+ (+ (`local.ConeBaseCentre`) (* (`local.TorchUp`) (`KismetMathLibrary.DegCos` _returnvalue))) (* (`local.TorchRight`) (`KismetMathLibrary.DegSin` _returnvalue))) (struct :`R` 0.917517 :`G` 0.984375 :`B` 0.208154 :`A` 1.0) 0.0 1.0))))

(fn `GetGunSocket`
  (bind _gunmuzzlesc (`/Game/FirstPersonCPP/Blueprints/FirstPersonCharacter.GetMuzzleSceneComponent` (`self.FPSController`)))
  (if (`KismetSystemLibrary.IsValid` _gunmuzzlesc)
    (`self.K2_AttachToComponent` _gunmuzzlesc "Muzzle" "SnapToTarget" "SnapToTarget" "KeepWorld" false)
    (else
      (`KismetSystemLibrary.PrintString` "NOOOOOOOOOOOOOOOOOO"))))

(fn `Toggle`
  (params (IsOn :type Boolean))
  (set `self.CurrentStartFOV` (`self.FOV`))
  (if IsOn
    (set `self.CurrentEndFOV` (`self.MaxFOV`))
    (else
      (set `self.CurrentEndFOV` 0.0)))
  (set `self.ElapsedWhileChangingFOV` 0.0))

(fn `UserConstructionScript`)